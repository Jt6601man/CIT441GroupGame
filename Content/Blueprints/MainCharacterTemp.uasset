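; Player character Blueprint with basic walk, turn, look and crouch-toggle controls, plus look-to-interact with objects in the world.
; Each tick, a short sphere trace from the camera tracks the hit actor as TracedObject, sending hover and unhover messages when it changes.
; The Activate input sends an activate message to that actor, and the trace draws its debug shape every frame.
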(event EventBeginPlay)

(event Collision|EventActorBeginOverlap
  (params (OtherActor :type Actor%20Object%20Reference)))

(event EventTick
  (params (DeltaSeconds :type Float%20%28single-precision%29))
  (bind _camera (Variables|Default|GetCamera))
  (bind _returnvalue (Transformation|GetWorldLocation _camera))
  ;[1 1 1] E to Activate
  (bind (_outhit _returnvalue_2) (Collision|SphereTraceByChannel _returnvalue (+ _returnvalue (* (Math|Vector|GetForwardVector _camera) 2.5e+02)) 2e+01 "TraceTypeQuery1" false 0 "ForOneFrame"))
  (if _returnvalue_2
    (if (!= (Variables|Default|GettracedObject) (.hitactor _outhit))
      (Class|IActivateable|UnHover(Message) (Variables|Default|GettracedObject))
      (bind _output_get (Variables|Default|SetTracedObject (.hitactor _outhit)))
      (Class|IActivateable|Hover(Message) _output_get))
    (else
      (Utilities|IsValid (Variables|Default|GetTracedObject)
        (:Is%20Valid
          (Class|IActivateable|UnHover(Message) (Variables|Default|GetTracedObject))
          (Variables|Default|SetTracedObject 0))))))

(event Input|ActionEvents|InputActionCrouch
  (params (Key :type Key%20Structure :default "None"))
  ;[1 1 1] Controls
  (:Pressed
    (if (Variables|Default|GetCrouched?)
      (Character|UnCrouch)
      (Variables|Default|SetCrouched? false)
      (else
        (Character|Crouch)
        (Variables|Default|SetCrouched? true)))))

(event Input|ActionEvents|InputActionActivate
  (params (Key :type Key%20Structure :default "None"))
  (bind _tracedobject (Variables|Default|GetTracedObject))
  ;[1 1 1] E to Activate
  (:Pressed
    (Utilities|IsValid _tracedobject
      (:Is%20Valid
        (Class|IActivateable|Activate(Message) _tracedobject)))))

(event Input|AxisEvents|InputAxisWalk
  (params (AxisValue :type Float%20%28single-precision%29))
  ;[1 1 1] Controls
  (Class|PawnMovementComponent|AddInputVector (Variables|Character|GetCharacterMovement) (* (Transformation|GetActorForwardVector) AxisValue) false))

(event Input|AxisEvents|InputAxisTurn
  (params (AxisValue :type Float%20%28single-precision%29))
  ;[1 1 1] Controls
  (Pawn|Input|AddControllerYawInput AxisValue))

(event Input|AxisEvents|InputAxisUpDown
  (params (AxisValue :type Float%20%28single-precision%29))
  ;[1 1 1] Controls
  (Pawn|Input|AddControllerPitchInput AxisValue))

(fn ConstructionScript)