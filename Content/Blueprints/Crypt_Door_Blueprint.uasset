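; Crypt door Blueprint that serves as the entrance to Level2, gated on whether the player has a flashlight.
; BeginPlay caches the MainCharacter, and Hover checks its HasFlashlight flag to show either an EnterCrypt or a TooDark prompt widget.
; UnHover removes that prompt, and Activate opens Level2 by name only when the character has the flashlight.
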(event EventUnHover
  (Widget|RemovefromParent (Variables|Default|GetactivateMessage)))

(event EventBeginPlay
  (bind _returnvalue (Actor|GetActorOfClass "/Game/Blueprints/MainCharacter.MainCharacter_C"))
  (Variables|Default|Setcharacter _returnvalue))

(event EventHover
  (if (Variables|/Game/Blueprints/MainCharacter.MainCharacter_C|GethasFlashlight (Variables|Default|Getcharacter))
    (bind _returnvalue (UserInterface|CreateWidget "/Game/Blueprints/Widgets/EnterCrypt.EnterCrypt_C"))
    (bind _output_get (Variables|Default|SetactivateMessage _returnvalue))
    (UserInterface|Viewport|AddtoViewport _output_get 0)
    (else
      (bind _returnvalue_2 (UserInterface|CreateWidget "/Game/Blueprints/Widgets/TooDark.TooDark_C"))
      (bind _output_get_2 (Variables|Default|SetactivateMessage _returnvalue_2))
      (UserInterface|Viewport|AddtoViewport _output_get_2 0))))

(event EventActivate
  (if (Variables|/Game/Blueprints/MainCharacter.MainCharacter_C|GethasFlashlight (Variables|Default|Getcharacter))
    (Game|OpenLevel(byName) "Level2")))

(fn ConstructionScript)