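; Safe is an interactable Blueprint that opens a combination entry screen when activated.
; Hover adds a PressToActivate prompt to the viewport and UnHover removes it.
; Activate creates the ComboEnter widget, shows the mouse cursor, switches to UI-only input focused on it, calls InMenu on the MainCharacter, then removes the prompt.
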(event EventUnHover
  (Widget|RemovefromParent (Variables|Default|GetactivateMessage)))

(event EventHover
  (bind _returnvalue (UserInterface|CreateWidget "/Game/Blueprints/Widgets/PressToActivate.PressToActivate_C"))
  (bind _output_get (Variables|Default|SetactivateMessage _returnvalue))
  (UserInterface|Viewport|AddtoViewport _output_get 0))

(event EventActivate
  (bind _returnvalue (Game|GetPlayerController 0))
  (bind _returnvalue_2 (UserInterface|CreateWidget "/Game/Blueprints/Widgets/ComboEnter.ComboEnter_C"))
  (UserInterface|Viewport|AddtoViewport _returnvalue_2 0)
  (Variables|/Script/Engine.PlayerController|SetbShowMouseCursor _returnvalue true)
  (Input|SetInputModeUIOnly _returnvalue _returnvalue_2 "DoNotLock")
  (bind _returnvalue_3 (Actor|GetActorOfClass "/Game/Blueprints/MainCharacter.MainCharacter_C"))
  (Default|InMenu _returnvalue_3)
  (Widget|RemovefromParent (Variables|Default|GetactivateMessage)))

(fn ConstructionScript)