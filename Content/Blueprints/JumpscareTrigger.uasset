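; JumpscareTrigger is a trigger actor that springs an ending jumpscare when the MainCharacter overlaps it.
; On overlap it turns off overlap events on its Box, adds a Static widget to the viewport, and calls PlayAllSounds to layer several loud 2D static, noise and alert sounds at once.
; After a short delay it opens the Credits level.
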(event Collision|EventActorBeginOverlap
  (params (OtherActor :type Actor%20Object%20Reference))
  (Utilities|Casting|CastToMainCharacter OtherActor)
  (Variables|/Script/Engine.PrimitiveComponent|SetbGenerateOverlapEvents (Variables|Default|GetBox) false)
  (bind _returnvalue (UserInterface|CreateWidget "/Game/JensenAssets/Static.Static_C"))
  (UserInterface|Viewport|AddtoViewport _returnvalue 0)
  (CallFunction|PlayAllSounds)
  (Utilities|FlowControl|Delay 5.0)
  (Game|OpenLevel(byName) "Credits"))

(fn ConstructionScript)

(fn PlayAllSounds
  (Audio|PlaySound2D "/Game/JensenAssets/171257__groovyrandomness__static.171257__groovyrandomness__static" 1.5 1.0 0.0 0 0)
  (Audio|PlaySound2D "/Game/JensenAssets/371183__doty21__corrupted-static-noise-loopable.371183__doty21__corrupted-static-noise-loopable" 1.5 1.0 0.0 0 0)
  (Audio|PlaySound2D "/Game/JensenAssets/sirednheadimitationsound.sirednheadimitationsound" 1.5 1.0 0.0 0 0)
  (Audio|PlaySound2D "/Game/JensenAssets/Weather_Emergency_Alert_Sound_Effect_wmv.Weather_Emergency_Alert_Sound_Effect_wmv" 1.5 1.0 0.0 0 0)
  (Audio|PlaySound2D "/Game/JensenAssets/169277__cognito-perceptu__static-750-traffic.169277__cognito-perceptu__static-750-traffic" 1.5 1.0 0.0 0 0))