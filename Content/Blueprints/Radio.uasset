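; Interactable radio the player can tune between frequencies to hear a correct signal, a spooky signal or static.
; Hover and UnHover toggle a prompt widget; Activate removes it, opens the ChangeFreq widget in UI-only input and calls InMenu on MainCharacter.
; Increment and Decrement play a blip and step the frequency within limits.
; ChangeFreq crossfades the Correct, Spooky and Noise audio by exact match against CorrectFreq and SpookyFreq.
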(event EventUnHover
  (Widget|RemovefromParent (Variables|Default|GetactivateMessage)))

(event EventBeginPlay)

(event EventHover
  (bind _returnvalue (UserInterface|CreateWidget "/Game/Blueprints/Widgets/PressToActivate.PressToActivate_C"))
  (bind _output_get (Variables|Default|SetactivateMessage _returnvalue))
  (UserInterface|Viewport|AddtoViewport _output_get 0))

(event EventActivate
  (bind _returnvalue (Game|GetPlayerController 0))
  (bind _returnvalue_2 (UserInterface|CreateWidget "/Game/Blueprints/Widgets/ChangeFreq.ChangeFreq_C" 0 self))
  (UserInterface|Viewport|AddtoViewport _returnvalue_2 0)
  (Variables|/Script/Engine.PlayerController|SetbShowMouseCursor _returnvalue true)
  (Input|SetInputModeUIOnly _returnvalue _returnvalue_2 "DoNotLock")
  (bind _returnvalue_3 (Actor|GetActorOfClass "/Game/Blueprints/MainCharacter.MainCharacter_C"))
  (Default|InMenu _returnvalue_3)
  (Widget|RemovefromParent (Variables|Default|GetactivateMessage)))

(fn ConstructionScript)

(fn Increment
  (Audio|PlaySoundatLocation "/Game/Audio/264590__vacuumfan7072__blip2.264590__vacuumfan7072__blip2" (Transformation|GetActorLocation) "0, 0, 0" 1.0 1.0 0.0 0 0 0)
  (if (< (Variables|Default|GetcurrFreq) 105.0)
    (CallFunction|ChangeFreq 2.5)))

(fn Decrement
  (Audio|PlaySoundatLocation "/Game/Audio/264590__vacuumfan7072__blip2.264590__vacuumfan7072__blip2" (Transformation|GetActorLocation) "0, 0, 0" 1.0 1.0 0.0 0 0 0)
  (if (> (Variables|Default|GetcurrFreq) 9e+01)
    (CallFunction|ChangeFreq -2.5)))

(fn ChangeFreq
  (params (change :type Float%20%28single-precision%29))
  (bind _correct (Variables|Default|GetCorrect))
  (bind _noise (Variables|Default|GetNoise))
  (bind _spooky (Variables|Default|GetSpooky))
  (bind _output_get (Variables|Default|SetcurrFreq (+ change (Variables|Default|GetcurrFreq))))
  (if (== _output_get (Variables|Default|GetcorrectFreq))
    (Audio|Components|Audio|AdjustVolume _correct 0.5 1e+02 "Linear" :!class /Script/Engine.AudioComponent)
    (Audio|Components|Audio|AdjustVolume _spooky 0.5 0.01 "Linear" :!class /Script/Engine.AudioComponent)
    (Audio|Components|Audio|AdjustVolume _noise 0.5 0.05 "Linear" :!class /Script/Engine.AudioComponent :!label _label)
    (elif (== _output_get (Variables|Default|GetspookyFreq))
      (Audio|Components|Audio|AdjustVolume _spooky 0.5 1e+02 "Linear" :!class /Script/Engine.AudioComponent)
      (Audio|Components|Audio|AdjustVolume _correct 0.5 0.01 "Linear" :!class /Script/Engine.AudioComponent)
      (goto _label)
      (else
        (Audio|Components|Audio|AdjustVolume _noise 0.5 1.0 "Linear" :!class /Script/Engine.AudioComponent)
        (Audio|Components|Audio|AdjustVolume _correct 0.5 0.01 "Linear" :!class /Script/Engine.AudioComponent)
        (Audio|Components|Audio|AdjustVolume _spooky 0.5 0.01 "Linear" :!class /Script/Engine.AudioComponent)))))