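; First-person player character for a Siren Head horror game, with movement, look, sprint, crouch toggle and an obtainable flashlight.
; A per-frame camera sphere trace, with debug drawing on, tracks the aimed actor and sends it hover and unhover messages; Activate messages that actor.
; InMenu disables input, halts SirenHeadPawn's timers, detection spheres and movement, and clears Static widgets.
; OutMenu restores input and spheres, then restarts the monster's wandering.
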(event EventBeginPlay
  (Rendering|SetVisibility (Variables|Default|GetFlashLight) false true))

(event Collision|EventActorBeginOverlap
  (params (OtherActor :type Actor%20Object%20Reference)))

(event EventTick
  (params (DeltaSeconds :type Float%20%28single-precision%29))
  (bind _camera (Variables|Default|GetCamera))
  (bind _returnvalue (Transformation|GetWorldLocation _camera))
  ;[1 1 1] Activatable
  (bind (_outhit _returnvalue_2) (Collision|SphereTraceByChannel _returnvalue (+ _returnvalue (* (Math|Vector|GetForwardVector _camera) 2.5e+02)) 2e+01 "TraceTypeQuery1" false 0 "ForOneFrame"))
  (if _returnvalue_2
    (if (!= (Variables|Default|GettracedObject) (.hitactor _outhit))
      (Class|IActivateable|UnHover(Message) (Variables|Default|GettracedObject))
      (bind _output_get (Variables|Default|SettracedObject (.hitactor _outhit)))
      (Class|IActivateable|Hover(Message) _output_get))
    (else
      (Utilities|IsValid (Variables|Default|GettracedObject)
        (:Is%20Valid
          (Class|IActivateable|UnHover(Message) (Variables|Default|GettracedObject))
          (Variables|Default|SettracedObject 0))))))

(event Input|ActionEvents|InputActionCrouch
  (params (Key :type Key%20Structure))
  ;[1 1 1] Controls
  (:Pressed
    (if (Variables|Default|GetCrouched?)
      (Character|UnCrouch)
      (Variables|Default|SetCrouched? false)
      (else
        (Character|Crouch)
        (Variables|Default|SetCrouched? true)))))

(event Input|ActionEvents|InputActionSprint
  (params (Key :type Key%20Structure))
  (bind _charactermovement (Variables|Character|GetCharacterMovement))
  ;[1 1 1] Controls
  (:Pressed
    (Variables|/Script/Engine.CharacterMovementComponent|SetMaxWalkSpeed _charactermovement 8e+02)
    (Character|UnCrouch)
    (Variables|Default|SetCrouched? false))
  (:Released
    (Variables|/Script/Engine.CharacterMovementComponent|SetMaxWalkSpeed _charactermovement 6e+02)))

(event Input|ActionEvents|InputActionFlashlight
  (params (Key :type Key%20Structure))
  ;[1 1 1] Controls
  (:Released
    (CallFunction|ToggleFlashlight)))

(event Input|ActionEvents|InputActionActivate
  (params (Key :type Key%20Structure))
  (bind _tracedobject (Variables|Default|GettracedObject))
  ;[1 1 1] Activatable
  (:Pressed
    (Utilities|IsValid _tracedobject
      (:Is%20Valid
        (Class|IActivateable|Activate(Message) _tracedobject)))))

(event Input|AxisEvents|InputAxisWalk
  (params (AxisValue :type Float%20%28single-precision%29))
  ;[1 1 1] Controls
  (Class|PawnMovementComponent|AddInputVector (Variables|Character|GetCharacterMovement) (* (Transformation|GetActorForwardVector) AxisValue) false))

(event Input|AxisEvents|InputAxisTurn
  (params (AxisValue :type Float%20%28single-precision%29))
  ;[1 1 1] Controls
  (Pawn|Input|AddControllerYawInput AxisValue))

(event Input|AxisEvents|InputAxisUpDown
  (params (AxisValue :type Float%20%28single-precision%29))
  ;[1 1 1] Controls
  (Pawn|Input|AddControllerPitchInput AxisValue))

(fn ConstructionScript)

(fn EnableFlashlight
  (Rendering|SetVisibility (Variables|Default|GetFlashLight) true true)
  (Variables|Default|SethasFlashlight true))

(fn ToggleFlashlight
  (if (Variables|Default|GethasFlashlight)
    (Rendering|ToggleVisibility (Variables|Default|GetSpotLight) false)
    (Audio|PlaySound2D "/Game/Audio/457458__rudmer-rotteveel__small-flashlight-click-on-01.457458__rudmer-rotteveel__small-flashlight-click-on-01" 1.5 1.0 0.0 0 0)))

(fn InMenu
  (Input|DisableInput 0)
  (Variables|Default|SetmenuActive true)
  ;[1 0.5099 0.2243] MonsterPauseCode
  (bind _returnvalue (Actor|GetActorOfClass "/Game/JensenAssets/SirenHeadPawn.SirenHeadPawn_C"))
  (bind _assiren_head_pawn (Utilities|Casting|CastToSirenHeadPawn _returnvalue))
  (Utilities|Time|PauseTimerbyHandle (Variables|/Game/JensenAssets/SirenHeadPawn.SirenHeadPawn_C|GetWanderTimer _assiren_head_pawn))
  (Utilities|Time|PauseTimerbyHandle (Variables|/Game/JensenAssets/SirenHeadPawn.SirenHeadPawn_C|GetChaseFunctionTimer _assiren_head_pawn))
  (Components|Activation|SetActive (Variables|/Game/JensenAssets/SirenHeadPawn.SirenHeadPawn_C|GetSphere _assiren_head_pawn) false false)
  (Variables|/Game/JensenAssets/SirenHeadPawn.SirenHeadPawn_C|SetTargetPoint _assiren_head_pawn (Transformation|GetActorLocation _assiren_head_pawn))
  (Variables|/Game/JensenAssets/SirenHeadPawn.SirenHeadPawn_C|SetDeathCounter _assiren_head_pawn 0)
  (Variables|/Game/JensenAssets/SirenHeadPawn.SirenHeadPawn_C|SetDeathZone _assiren_head_pawn false)
  (Class|NavMovementComponent|StopActiveMovement (Variables|/Game/JensenAssets/SirenHeadPawn.SirenHeadPawn_C|GetFloatingPawnMovement _assiren_head_pawn))
  (bind _foundwidgets (Widget|GetAllWidgetsOfClass "/Game/JensenAssets/Static.Static_C" true))
  (Widget|RemovefromParent _foundwidgets))

(fn OutMenu
  (Input|EnableInput 0)
  (Variables|Default|SetmenuActive false)
  ;[1 0.5099 0.2243] MonsterUnPauseCode
  (bind _returnvalue (Actor|GetActorOfClass "/Game/JensenAssets/SirenHeadPawn.SirenHeadPawn_C"))
  (bind _assiren_head_pawn (Utilities|Casting|CastToSirenHeadPawn _returnvalue))
  (Components|Activation|SetActive (Variables|/Game/JensenAssets/SirenHeadPawn.SirenHeadPawn_C|GetSphere _assiren_head_pawn) true false)
  (Default|WandertoRandomPoint _assiren_head_pawn))